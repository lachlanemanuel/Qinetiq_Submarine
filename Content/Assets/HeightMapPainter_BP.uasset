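; Height map painter Blueprint that prepares painting resources and finds the UV point under the player's camera aim.
; The construction script creates an RGBA16f heightfield render target, a paint material instance for its static mesh and a splat material instance.
; TraceFromCamera line-traces along the view, stores the hit's collision UV and sends point damage to the hit actor.
; The file contains no render target drawing or calls to the trace.
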(fn `TraceFromCamera`
  (bind _returnvalue (`GameplayStatics.GetPlayerCameraManager` 0))
  (bind _returnvalue_2 (`self.K2_GetActorLocation` _returnvalue))
  (bind (_outhit _returnvalue_3) (`KismetSystemLibrary.LineTraceSingle` _returnvalue_2 (+ (* (`KismetMathLibrary.Normal` (`KismetMathLibrary.Conv_RotatorToVector` (`self.K2_GetActorRotation` _returnvalue))) (* (`self.InteractionDistance`) 10.0)) _returnvalue_2) "TraceTypeQuery1" true))
  (if _returnvalue_3
    (bind (_bblockinghit _binitialoverlap _time _distance _location _impactpoint _normal _impactnormal _physmat _hitactor) (`GameplayStatics.BreakHitResult` _outhit))
    (`/Engine/EditorBlueprintResources/StandardMacros.IsValid` _hitactor
      (:`Is Valid`
        (set `self.CollisionUVHit` (`GameplayStatics.FindCollisionUV` _outhit))
        (`GameplayStatics.ApplyPointDamage` _hitactor 0.0 (`KismetMathLibrary.MakeVector` 0.0 0.0 1.0) (struct) (`GameplayStatics.GetPlayerController` 0))))))

(fn `UserConstructionScript`
  (bind _returnvalue (`KismetRenderingLibrary.CreateRenderTarget2D` (`self.RT_W_Size`) (`self.RT_H_Size`)))
  (set `self.Heightfield_RT` _returnvalue)
  (bind _returnvalue_2 (`KismetMaterialLibrary.CreateDynamicMaterialInstance` "/Game/Assets/HeightMapPaint_MasterMaterial.HeightMapPaint_MasterMaterial"))
  (bind _output_get (set `self.Painter_MI` _returnvalue_2))
  (`PrimitiveComponent.SetMaterial` (`self.StaticMeshComponent`) 0 _output_get)
  (bind _returnvalue_3 (`KismetMaterialLibrary.CreateDynamicMaterialInstance` "/Game/Assets/Splat_MasterMaterial.Splat_MasterMaterial"))
  (set `self.ForceSpaltMID` _returnvalue_3))